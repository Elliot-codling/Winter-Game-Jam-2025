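; BP_Computer is a focusable computer terminal actor whose screen is a terminal UI in a widget component.
; It extends its parent's focus states, activating the terminal screen widget when focus is entered.
; While focused, each tick forces keyboard focus onto that widget.
; Leaving focus sets viewport mouse capture to capture during mouse down.
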(event `self.ReceiveBeginPlay`
  (`parent.ReceiveBeginPlay`))

(fn `EnterFocusedState`
  (`parent.EnterFocusedState`)
  (bind _asuwb_terminal_screen (cast `/Game/Focusables/Terminal/UWB_TerminalScreen` (`WidgetComponent.GetUserWidgetObject` (`self.ScreenWidget`))))
  (`/Game/Focusables/Terminal/UWB_TerminalScreen.SetActive` _asuwb_terminal_screen))

(fn `ExitFocusState`
  (`parent.ExitFocusState`)
  (`GameplayStatics.SetViewportMouseCaptureMode` "CaptureDuringMouseDown"))

(fn `TickFocusedState`
  (`parent.TickFocusedState`)
  (`Widget.SetKeyboardFocus` (`WidgetComponent.GetUserWidgetObject` (`self.ScreenWidget`))))

(fn `UserConstructionScript`
  (`parent.UserConstructionScript`))