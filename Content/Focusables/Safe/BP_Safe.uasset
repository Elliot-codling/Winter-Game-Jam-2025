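; BP_Safe is a focusable safe with a keypad whose correct code completes the game.
; GetComponentHit reads the hit component's object name as the key: digits append to Password, Clear empties it, and Submit calls SubmitPassword.
; A match with CorrectPassword sets PasswordUnlocked, exposed through HasSafeUnlocked, and shows the BP_GameComplete widget, while a wrong code resets the entry.
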(event `GetComponentHit`
  (params (HitResult :type "HitResult Structure"))
  (bind _returnvalue (`KismetSystemLibrary.GetObjectName` (`.HitComponent` (`GameplayStatics.BreakHitResult` HitResult))))
  ;[1 1 1] Get key on keypad that was hit and append that to the password
  (switch `string` _returnvalue
    (:`0`
      (bind _output_get (set `self.Password` (`KismetStringLibrary.Concat_StrStr` (`self.Password`) _returnvalue) :!label _label))
      (`KismetSystemLibrary.PrintString` _output_get :!label _label_2))
    (:`1`
      (goto _label))
    (:`2`
      (goto _label))
    (:`3`
      (goto _label))
    (:`4`
      (goto _label))
    (:`5`
      (goto _label))
    (:`6`
      (goto _label))
    (:`7`
      (goto _label))
    (:`8`
      (goto _label))
    (:`9`
      (goto _label))
    (:`Clear`
      (set `self.Password` "")
      (goto _label_2))
    (:`Submit`
      ;;[1 1 1] Do Level Completion Logic Here
      (`self.SubmitPassword`))))

(event `SubmitPassword`
  ;[1 1 1] Submit Password
  (if (`KismetStringLibrary.EqualEqual_StrStr` (`self.Password`) (`self.CorrectPassword`))
    (set `self.PasswordUnlocked` true)
    (bind _returnvalue (`|CreateWidget` "/Game/Player/BP_GameComplete.BP_GameComplete_C"))
    (`UserWidget.AddToViewport` _returnvalue 0)
    (else
      (set `self.Password` ""))))

(fn `HasSafeUnlocked`
  (returns (Value :type Boolean))
  (return (`self.PasswordUnlocked`)))

(fn `UserConstructionScript`
  (`parent.UserConstructionScript`))