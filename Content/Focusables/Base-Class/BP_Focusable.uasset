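; BP_Focusable is a base Blueprint for focusable objects, tagged Focusable and set to NotFocused on BeginPlay.
; ChangeState is a simple enum state machine that runs an exit switch when the state differs, then stores the state, resets elapsed time and runs an enter switch.
; All state branches are empty stubs with debug prints, and the per-state update and timer logic is disconnected from Tick.
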(event `self.ReceiveBeginPlay`
  (`BlueprintGameplayTagLibrary.AddGameplayTag` (`BlueprintGameplayTagLibrary.MakeGameplayTagContainerFromTag` (struct :`TagName` "Focusable")) (struct :`TagName` "Focusable"))
  (`self.ChangeState` "NewEnumerator1"))

(event `self.ReceiveTick`
  (params (DeltaSeconds :type "Float (single-precision)")))

(fn `ChangeState`
  (params (newState :type "/Game/Focusables/Base-Class/E_FocusState Enum" :default "NewEnumerator0"))
  (if (not (`|EnumEquality` newState (`self.currentFocusState`)))
    (switch `/Game/Focusables/Base-Class/E_FocusState` (`self.currentFocusState`)
      (:`NewEnumerator0`
        _)
      (:`NewEnumerator1`
        _))
    (`KismetSystemLibrary.PrintString` "Exit"))
  (set `self.currentFocusState` newState)
  (set `self.elapsedTimeInState` 0.0)
  (switch `/Game/Focusables/Base-Class/E_FocusState` (`self.currentFocusState`)
    (:`NewEnumerator0`
      _)
    (:`NewEnumerator1`
      _))
  (`KismetSystemLibrary.PrintString` "Enter"))

(fn `UserConstructionScript`)