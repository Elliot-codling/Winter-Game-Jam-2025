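; BP_BookSlot is a slot in the bookcase puzzle that tracks whether it is filled and which colour it holds (None, Red, Blue or Green).
; CallParent casts its attach-parent actor to BP_BookcasePuzzle and passes itself to that puzzle's SlotCheck.
; ChangeSlotFilledState and ChangeSlotColourState are simple enum state machines whose exit and enter branches currently only print debug strings.
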(event `CallParent`
  (bind _asbp_bookcase_puzzle (cast `/Game/BookcaseBackupSolution/BP_BookcasePuzzle` (`self.GetAttachParentActor`)))
  (`KismetSystemLibrary.PrintString` "Got Parent!")
  (`/Game/BookcaseBackupSolution/BP_BookcasePuzzle.SlotCheck` _asbp_bookcase_puzzle self))

(fn `ChangeSlotColourState`
  (params (newState :type "/Game/BookcaseBackupSolution/E_ColourState Enum" :default "NewEnumerator0"))
  ;[1 1 1] Check if current state is not equal to new state
  (if (not (`|EnumEquality` newState (`self.currentColourState`)))
    ;[1 1 1] Exit State
    (switch `/Game/BookcaseBackupSolution/E_ColourState` (`self.currentColourState`)
      (:`NewEnumerator3`
        (`KismetSystemLibrary.PrintString` "Exit None"))
      (:`NewEnumerator0`
        (`KismetSystemLibrary.PrintString` "Exit Red"))
      (:`NewEnumerator1`
        (`KismetSystemLibrary.PrintString` "Exit Blue"))
      (:`NewEnumerator2`
        (`KismetSystemLibrary.PrintString` "Exit Green"))))
  (set `self.currentColourState` newState)
  ;[1 1 1] Enter New State
  (switch `/Game/BookcaseBackupSolution/E_ColourState` (`self.currentColourState`)
    (:`NewEnumerator3`
      (`KismetSystemLibrary.PrintString` "Enter None"))
    (:`NewEnumerator0`
      (`KismetSystemLibrary.PrintString` "Enter Red"))
    (:`NewEnumerator1`
      (`KismetSystemLibrary.PrintString` "Enter Blue"))
    (:`NewEnumerator2`
      (`KismetSystemLibrary.PrintString` "Enter Green"))))

(fn `ChangeSlotFilledState`
  (params (newState :type "/Game/BookcaseBackupSolution/E_SlotState Enum" :default "NewEnumerator0"))
  ;[1 1 1] Check if current state is not equal to new state
  (if (not (`|EnumEquality` newState (`self.currentFilledState`)))
    ;[1 1 1] Exit State
    (switch `/Game/BookcaseBackupSolution/E_SlotState` (`self.currentFilledState`)
      (:`NewEnumerator0`
        (`KismetSystemLibrary.PrintString` "Exit Filled"))
      (:`NewEnumerator1`
        (`KismetSystemLibrary.PrintString` "Exit Empty"))))
  (set `self.currentFilledState` newState)
  ;[1 1 1] Enter New State
  (switch `/Game/BookcaseBackupSolution/E_SlotState` (`self.currentFilledState`)
    (:`NewEnumerator0`
      (`KismetSystemLibrary.PrintString` "Enter Filled"))
    (:`NewEnumerator1`
      (`KismetSystemLibrary.PrintString` "Enter Empty"))))

(fn `UserConstructionScript`)