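; BP_BookcasePuzzle is the parent actor for a bookcase puzzle made up of BP_BookSlot child actors.
; On BeginPlay it stores its child slots in a BookSlots array in child-actor order.
; SlotCheck prints the given slot's index in that array, then sets that slot's filled and colour states to fixed values.
; No validation or win condition is implemented here.
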(event `self.ReceiveBeginPlay`
  ;[1 1 1] Add all children to array
  (for (_array_element _array_index) (`self.GetAllChildActors` true)
    (bind _asbp_book_slot (cast `/Game/BookcaseBackupSolution/BP_BookSlot` _array_element))
    (`KismetArrayLibrary.Array_Set` (`self.bookSlots`) _array_index _asbp_book_slot)))

(event `SlotCheck`
  (params (Slot :type "/Game/BookcaseBackupSolution/BP_BookSlot Object Reference"))
  (`KismetSystemLibrary.PrintString` (`KismetStringLibrary.Conv_IntToString` (`KismetArrayLibrary.Array_Find` (`self.bookSlots`) Slot)))
  (`/Game/BookcaseBackupSolution/BP_BookSlot.ChangeSlotFilledState` Slot "NewEnumerator0")
  (`/Game/BookcaseBackupSolution/BP_BookSlot.ChangeSlotColourState` Slot "NewEnumerator1"))

(fn `UserConstructionScript`)