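; BP_RedBook_Placeable is a collectable book placement actor that, despite its name, can display a red, green or blue book.
; All three book components start hidden; ShowBook and HideBook toggle the one matching the passed index and return whether state changed.
; A single BookVisibility flag limits it to one book.
; ShowBook records ColorID even when already occupied, and getters expose both values.
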(event `self.ReceiveBeginPlay`
  (`|ExecutionSequence`
    (:`then_0`
      (`SceneComponent.SetVisibility` (`self.BP_Red_Book_Corners`) false false))
    (:`then_1`
      (`SceneComponent.SetVisibility` (`self.BP_Green_Book_Corners`) false false))
    (:`then_2`
      (`SceneComponent.SetVisibility` (`self.BP_Blue_Book_Corners`) false false))))

(fn `GetColorID`
  (returns (ColorID :type Integer))
  (return (`self.ColorID`)))

(fn `HideBook`
  (params (BookActorIndex :type Integer))
  (returns (HasBookBeenRemoved :type Boolean))
  (set `self.BookChangedState` false)
  (if (`self.BookVisibility`)
    (`|ExecutionSequence`
      (:`then_0`
        (if (== BookActorIndex 0)
          (`SceneComponent.SetVisibility` (`self.BP_Red_Book_Corners`) false false)
          (set `self.BookVisibility` false :!label _label)
          (set `self.BookChangedState` true)
          (return (`self.BookChangedState`))))
      (:`then_1`
        (if (== BookActorIndex 1)
          (`SceneComponent.SetVisibility` (`self.BP_Green_Book_Corners`) false false)
          (goto _label)))
      (:`then_2`
        (if (== BookActorIndex 2)
          (`SceneComponent.SetVisibility` (`self.BP_Blue_Book_Corners`) false false)
          (goto _label))))
    (else
      (return (`self.BookChangedState`)))))

(fn `IsBookVisable`
  (returns (Value :type Boolean))
  (return (`self.BookVisibility`)))

(fn `ShowBook`
  (params (BookActorIndex :type Integer))
  (returns (HasBookBeenPlaced :type Boolean))
  (set `self.ColorID` BookActorIndex)
  (set `self.BookChangedState` false)
  (if (`self.BookVisibility`)
    (return (`self.BookChangedState`))
    (else
      (`|ExecutionSequence`
        (:`then_0`
          (if (== BookActorIndex 0)
            (`SceneComponent.SetVisibility` (`self.BP_Red_Book_Corners`) true false)
            (set `self.BookVisibility` true :!label _label)
            (set `self.BookChangedState` true)
            (return (`self.BookChangedState`))))
        (:`then_1`
          (if (== BookActorIndex 1)
            (`SceneComponent.SetVisibility` (`self.BP_Green_Book_Corners`) true false)
            (goto _label)))
        (:`then_2`
          (if (== BookActorIndex 2)
            (`SceneComponent.SetVisibility` (`self.BP_Blue_Book_Corners`) true false)
            (goto _label)))))))

(fn `UserConstructionScript`)