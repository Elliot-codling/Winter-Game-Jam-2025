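; Player camera actor that moves between a room overview and close-up views of clickable BP_Focusable objects.
; Left-click, when unfocused, line traces from the mouse cursor, changes the hit focusable's state and stores it as the current focus; R releases it.
; Tick eases the actor toward the focus's view position and look-at point, or back to the room base transform, using fixed-alpha lerps independent of delta time.
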(event `self.ReceiveTick`
  (params (DeltaSeconds :type "Float (single-precision)"))
  ;[1 1 1] Update Loop
  (if (`self.isFocused`)
    (`self.LerpCameraRotation`)
    (`self.LerpCameraPosition`)
    (else
      (`self.LerpCameraRotationBase`)
      (`self.LerpCameraPositionBase`))))

(event `LerpCameraPositionBase`
  (bind _returnvalue_location (`KismetMathLibrary.BreakTransform` (`KismetMathLibrary.TLerp` (`KismetMathLibrary.Conv_VectorToTransform` (`SceneComponent.K2_GetComponentLocation` (`self.Camera`))) (`KismetMathLibrary.Conv_VectorToTransform` (`self.roomBasePosition`)) 0.05)))
  ;[1 1 1] Lerp Position Base
  (`self.K2_SetActorLocation` _returnvalue_location))

(event `LerpCameraRotationBase`
  ;[1 1 1] Lerp Rotation Base
  (`self.K2_SetActorRotation` (`KismetMathLibrary.RLerp` (`SceneComponent.K2_GetComponentRotation` (`self.Camera`)) (`self.roomBaseRotation`) 0.05)))

(event `LerpCameraPosition`
  (bind _returnvalue_location (`KismetMathLibrary.BreakTransform` (`KismetMathLibrary.TLerp` (`KismetMathLibrary.Conv_VectorToTransform` (`SceneComponent.K2_GetComponentLocation` (`self.Camera`))) (`KismetMathLibrary.Conv_VectorToTransform` (`SceneComponent.K2_GetComponentLocation` (`/Game/Focusables/Base-Class/BP_Focusable.ViewPosition` (`self.currentFocus`)))) 0.05)))
  ;[1 1 1] Lerp Position
  (`self.K2_SetActorLocation` _returnvalue_location))

(event `LerpCameraRotation`
  (bind _camera (`self.Camera`))
  ;[1 1 1] Lerp Rotation
  (`self.K2_SetActorRotation` (`KismetMathLibrary.RLerp` (`SceneComponent.K2_GetComponentRotation` _camera) (`KismetMathLibrary.FindLookAtRotation` (`SceneComponent.K2_GetComponentLocation` _camera) (`SceneComponent.K2_GetComponentLocation` (`/Game/Focusables/Base-Class/BP_Focusable.FocusPoint` (`self.currentFocus`)))) 0.09 true)))

(event `Key|LeftMouseButton`
  (params (Key :type "Key Structure"))
  (bind (_worldlocation _worlddirection) (`PlayerController.DeprojectMousePositionToWorld` (`GameplayStatics.GetPlayerController` 0)))
  ;[1 1 1] Line Raycast
  (:`Pressed`
    (if (not (`self.isFocused`))
      (bind _outhit (`KismetSystemLibrary.LineTraceSingle` _worldlocation (+ _worldlocation (* _worlddirection 1000.0)) "TraceTypeQuery1"))
      (bind _asbp_focusable (cast `/Game/Focusables/Base-Class/BP_Focusable` (`.HitActor` (`GameplayStatics.BreakHitResult` _outhit))))
      (`/Game/Focusables/Base-Class/BP_Focusable.ChangeState` _asbp_focusable "NewEnumerator0")
      (set `self.currentFocus` _asbp_focusable)
      (set `self.isFocused` true))))

(event `Key|R`
  (params (Key :type "Key Structure"))
  ;[1 1 1] Reset Camera
  (:`Pressed`
    (if (`self.isFocused`)
      (`/Game/Focusables/Base-Class/BP_Focusable.ChangeState` (`self.currentFocus`) "NewEnumerator1")
      (set `self.currentFocus` null)
      (set `self.isFocused` false))))

(fn `UserConstructionScript`)